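; BP_RockNPCHouse is a house prop, apparently a quest reward, that visually rebuilds a broken NPC house when RebuildStructure is called.
; The event shows both house meshes and the dust component, plays construction sounds, then starts a timeline that fades opacity and lerps the meshes into place.
; Late in the timeline it repeatedly triggers camera shake, hides the broken mesh and plays a one-time drop sound.
; On finish, it hides the dust and swaps in final materials.
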(event `self.ReceiveBeginPlay`
  (`FXSystemComponent.SetEmitterEnable` (`self.PS_BuildingDust`) "None" false))

(event `RebuildStructure`
  (bind _small_house_low_outer_house_low (`self.Small_House_Low_Outer_House_Low`))
  (bind _returnvalue (`SceneComponent.K2_GetComponentLocation` (`self.House`)))
  (`SceneComponent.SetVisibility` (`self.House`) true true)
  (`SceneComponent.SetVisibility` (`self.Small_House_Low_Outer_House_Low`) true true)
  (`SceneComponent.SetVisibility` (`self.PS_BuildingDust`) true true)
  (`GameplayStatics.PlaySoundAtLocation` "/Game/Sounds/newSounds/SawCut.SawCut" _returnvalue (struct) 1.0 1.0 0.0 null null null)
  (`GameplayStatics.PlaySoundAtLocation` "/Game/Sounds/newSounds/HamerHit.HamerHit" _returnvalue (struct) 1.0 1.0 0.0 null null null)
  (bind (_direction _newtrack_0) (`Timeline|RebuildHouse`)
    (:`Update`
      (`MeshComponent.SetScalarParameterValueOnMaterials` (`self.House`) "Opacity" _newtrack_0)
      (`MeshComponent.SetScalarParameterValueOnMaterials` (`self.Small_House_Low_Outer_House_Low`) "Opacity" _newtrack_0)
      (bind _returnvalue_2 (`KismetMathLibrary.VLerp` (`self.NewVar_0`) (0.0 0.0 0.0) _newtrack_0))
      (`SceneComponent.K2_SetRelativeLocation` (`self.House`) _returnvalue_2 false false)
      (`SceneComponent.K2_SetRelativeLocation` _small_house_low_outer_house_low _returnvalue_2 false false)
      (if (and (> 0.99 _newtrack_0) (> _newtrack_0 0.6))
        (`GameplayStatics.PlayWorldCameraShake` "/Game/BP_CameraaShakeControl.BP_CameraaShakeControl_C" (`SceneComponent.K2_GetComponentLocation` _small_house_low_outer_house_low) 10000.0 10000.0 0.5)
        (`SceneComponent.SetVisibility` (`self.Broken_House_FBX`) false false)
        (`/Engine/EditorBlueprintResources/StandardMacros.DoOnce` false
          (:`Completed`
            (`GameplayStatics.PlaySoundAtLocation` "/Game/Sounds/newSounds/SFX_HouseDrop.SFX_HouseDrop" (`SceneComponent.K2_GetComponentLocation` (`self.House`)) (struct) 1.0 1.0 0.0 null null null)))))
    (:`Finished`
      (`SceneComponent.SetVisibility` (`self.PS_BuildingDust`) false true)
      (`PrimitiveComponent.SetMaterial` (`self.House`) 0 "/Game/Assets/City/SmalHouse/M_SmallHouse.M_SmallHouse")
      (`PrimitiveComponent.SetMaterial` (`self.Small_House_Low_Outer_House_Low`) 0 "/Game/Assets/City/SmalHouse/M_SmallHouseOut.M_SmallHouseOut"))))

(fn `UserConstructionScript`)