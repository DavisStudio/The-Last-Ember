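; BP_BirchTreeFoal is a birch tree world prop that leaves a log behind when destroyed.
; On BeginPlay it varies its Cylinder component with a slight random tilt, a random yaw and random per-axis scale.
; On Destroyed it spawns a BP_DestroyableProp_Log at the actor's transform and plays the TreFall sound there.
; The construction script only calls the parent's.
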(event `self.ReceiveDestroyed`
  (`|SpawnActorFromClass` "/Game/BluePrints/InWorldProps/Trees/BP_DestroyableProp_Log.BP_DestroyableProp_Log_C" (`self.GetTransform`) "AdjustIfPossibleButAlwaysSpawn" "OverrideRootScale" null null)
  (`GameplayStatics.PlaySoundAtLocation` "/Game/Sounds/TreFall.TreFall" (`self.K2_GetActorLocation`) (struct) 1.0 1.0 0.0 null null null))

(event `self.ReceiveBeginPlay`
  (bind _returnvalue (`KismetMathLibrary.RandomFloatInRange` 0.9 2.3))
  (`SceneComponent.K2_SetRelativeRotation` (`self.Cylinder`) (`KismetMathLibrary.MakeRotator` (`KismetMathLibrary.RandomFloatInRange` -7.0 7.0) (`KismetMathLibrary.RandomFloatInRange` -7.0 7.0) (`KismetMathLibrary.Conv_IntToDouble` (`KismetMathLibrary.RandomInteger` 360))) false false)
  (`SceneComponent.SetRelativeScale3D` (`self.Cylinder`) (`KismetMathLibrary.MakeVector` _returnvalue _returnvalue _returnvalue)))

(fn `UserConstructionScript`
  (`parent.UserConstructionScript`))