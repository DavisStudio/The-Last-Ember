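; BP_DestroyableProp_Log is a log prop that gives impact feedback when it hits the floor.
; On BeginPlay it runs the parent logic and assigns its Cylinder to PropMesh.
; Overlaps on either of two sphere components share one check for a "floor" tag, then play a world camera shake with a very large radius and a TreeSmack sound at the Cylinder's location.
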(event `self.ReceiveBeginPlay`
  (`parent.ReceiveBeginPlay`)
  (set `self.PropMesh` (`self.Cylinder`)))

(event `self.Sphere1.OnComponentBeginOverlap`
  (params (OverlappedComponent :type "PrimitiveComponent Object Reference") (OtherActor :type "Actor Object Reference") (OtherComp :type "PrimitiveComponent Object Reference") (OtherBodyIndex :type Integer) (bFromSweep :type Boolean) (SweepResult :type "HitResult Structure (by ref)"))
  (bind _returnvalue (`SceneComponent.K2_GetComponentLocation` (`self.Cylinder`)))
  (if (or (`self.ActorHasTag` OtherActor "floor") (`self.ActorHasTag` (stale `self.Sphere.OnComponentBeginOverlap` OtherActor) "floor")) :!label _label
    (`GameplayStatics.PlayWorldCameraShake` "/Game/BP_CameraaShakeControl.BP_CameraaShakeControl_C" _returnvalue 0.0 5000000.0)
    (`GameplayStatics.PlaySoundAtLocation` "/Game/Sounds/TreeSmack.TreeSmack" _returnvalue (struct) 1.0 1.0 0.0 null null null)))

(event `self.Sphere.OnComponentBeginOverlap`
  (params (OverlappedComponent :type "PrimitiveComponent Object Reference") (OtherActor :type "Actor Object Reference") (OtherComp :type "PrimitiveComponent Object Reference") (OtherBodyIndex :type Integer) (bFromSweep :type Boolean) (SweepResult :type "HitResult Structure (by ref)"))
  (goto _label))

(fn `UserConstructionScript`
  (`parent.UserConstructionScript`))