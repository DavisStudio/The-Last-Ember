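; BP_OakTreees is an oak tree world prop that turns into a log when destroyed.
; On BeginPlay it gives the Cylinder component a random whole-degree yaw for visual variety, keeping its world roll and pitch as relative values.
; On Destroyed it spawns BP_DestroyableProp_Log at the tree's transform, adjusting for collisions but always spawning, and plays the TreFall sound there.
; The construction script only calls the parent's.
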(event `self.ReceiveDestroyed`
  (`|SpawnActorFromClass` "/Game/BluePrints/InWorldProps/Trees/BP_DestroyableProp_Log.BP_DestroyableProp_Log_C" (`self.GetTransform`) "AdjustIfPossibleButAlwaysSpawn" "OverrideRootScale" null null)
  (`GameplayStatics.PlaySoundAtLocation` "/Game/Sounds/TreFall.TreFall" (`self.K2_GetActorLocation`) (struct) 1.0 1.0 0.0 null null null))

(event `self.ReceiveBeginPlay`
  (bind _cylinder (`self.Cylinder`))
  (bind (_returnvalue_roll _returnvalue_pitch) (`KismetMathLibrary.BreakRotator` (`SceneComponent.K2_GetComponentRotation` _cylinder)))
  (`SceneComponent.K2_SetRelativeRotation` _cylinder (`KismetMathLibrary.MakeRotator` _returnvalue_roll _returnvalue_pitch (`KismetMathLibrary.Conv_IntToDouble` (`KismetMathLibrary.RandomInteger` 360))) false false))

(fn `UserConstructionScript`
  (`parent.UserConstructionScript`))