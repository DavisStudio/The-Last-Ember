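; BP_Destroyable_Stone is a stone prop whose name marks it as destroyable, with its destruction handling left to the parent class.
; On BeginPlay it assigns its Cube component to PropMesh, then gives that mesh a random whole-degree yaw for visual variety.
; The rotation is set as relative but reuses roll and pitch read from world rotation.
; Destroyed and the construction script only call their parent versions.
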(event `self.ReceiveBeginPlay`
  (`parent.ReceiveBeginPlay`)
  (bind _output_get (set `self.PropMesh` (`self.Cube`)))
  (bind (_returnvalue_roll _returnvalue_pitch) (`KismetMathLibrary.BreakRotator` (`SceneComponent.K2_GetComponentRotation` _output_get)))
  (`SceneComponent.K2_SetRelativeRotation` _output_get (`KismetMathLibrary.MakeRotator` _returnvalue_roll _returnvalue_pitch (`KismetMathLibrary.Conv_IntToDouble` (`KismetMathLibrary.RandomInteger` 360))) false false))

(event `self.ReceiveDestroyed`
  (`parent.ReceiveDestroyed`))

(fn `UserConstructionScript`
  (`parent.UserConstructionScript`))