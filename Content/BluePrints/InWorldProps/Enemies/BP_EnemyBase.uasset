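; Base enemy Blueprint, built on prop data, that takes damage and drops loot when destroyed.
; TakeDamage subtracts from Health in the Properties struct, prints a debug value and destroys the actor when the health check falls below one.
; The Destroyed event spawns the first ItemDrops class above PropMesh and sets its item amount to a random value within the first MinMaxDropAmount range.
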(event `self.ReceiveDestroyed`
  (bind (_returnvalue_location _returnvalue_rotation _returnvalue_scale) (`KismetMathLibrary.BreakTransform` (`self.GetTransform`)))
  (bind (_properties_health _properties_maxhealth _properties_itemdrops _properties_minmaxdropamount) (break `/Game/BluePrints/Structs/ST_Prop` (`self.Properties`)))
  (bind _returnvalue (`|SpawnActorFromClass` (`|GetArrayItem` _properties_itemdrops) (`KismetMathLibrary.MakeTransform` (+ (`SceneComponent.K2_GetComponentLocation` (`self.PropMesh`)) (0.0 0.0 250.0)) _returnvalue_rotation _returnvalue_scale) "AdjustIfPossibleButAlwaysSpawn" "OverrideRootScale" null null))
  (setmembers `/Game/BluePrints/Structs/ST_Item` :`StructRef` (`/Game/BluePrints/Items/BP_Item.Properties` _returnvalue) :`Amount` (`KismetMathLibrary.RandomIntegerInRange` (`|GetArrayItem` _properties_minmaxdropamount) (`|GetArrayItem` _properties_minmaxdropamount 1))))

(fn `TakeDamage`
  (params (Damage :type "Float (double-precision)"))
  (bind _properties (`self.Properties`))
  (bind _returnvalue (- (`.Health_3_5170E67D4EBA095C82995681469B2943` (break `/Game/BluePrints/Structs/ST_Prop` _properties)) Damage))
  (setmembers `/Game/BluePrints/Structs/ST_Prop` :`StructRef` _properties :`Health` _returnvalue)
  (`KismetSystemLibrary.PrintString` (`KismetStringLibrary.Conv_DoubleToString` _returnvalue))
  (if (< _returnvalue 1.0)
    (`self.K2_DestroyActor`)))

(fn `UserConstructionScript`)