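; BP_Raat is an in-world prop enemy that chases the player character while it is inside a detection box and heads back to its start location otherwise.
; Box overlaps set or clear PlayerTarget, which Tick uses to pick the destination.
; MoveTowards sweeps the Cube there with a fixed-alpha lerp each frame, so speed depends on frame rate and distance.
; Cube overlaps only print the other actor's name.
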(event `self.ReceiveDestroyed`
  (`parent.ReceiveDestroyed`))

(event `self.ReceiveBeginPlay`
  (`parent.ReceiveBeginPlay`)
  (set `self.PropMesh` (`self.Cube`))
  (set `self.StartLocation` (`SceneComponent.K2_GetComponentLocation` (`self.Cube`))))

(event `self.ReceiveTick`
  (params (DeltaSeconds :type "Float (single-precision)"))
  (if (!= (`self.PlayerTarget`) null)
    (`self.MoveTowards` (`SceneComponent.K2_GetComponentLocation` (`Character.Mesh` (`self.PlayerTarget`))))
    (else
      (`self.MoveTowards` (`self.StartLocation`)))))

(event `self.Box.OnComponentBeginOverlap`
  (params (OverlappedComponent :type "PrimitiveComponent Object Reference") (OtherActor :type "Actor Object Reference") (OtherComp :type "PrimitiveComponent Object Reference") (OtherBodyIndex :type Integer) (bFromSweep :type Boolean) (SweepResult :type "HitResult Structure (by ref)"))
  (bind _asbp_charachter (cast `/Game/Charachter/BP_Charachter` OtherActor))
  (set `self.PlayerTarget` _asbp_charachter))

(event `self.Box.OnComponentEndOverlap`
  (params (OverlappedComponent :type "PrimitiveComponent Object Reference") (OtherActor :type "Actor Object Reference") (OtherComp :type "PrimitiveComponent Object Reference") (OtherBodyIndex :type Integer))
  (cast `/Game/Charachter/BP_Charachter` OtherActor)
  (set `self.PlayerTarget` null))

(event `self.Cube.OnComponentBeginOverlap`
  (params (OverlappedComponent :type "PrimitiveComponent Object Reference") (OtherActor :type "Actor Object Reference") (OtherComp :type "PrimitiveComponent Object Reference") (OtherBodyIndex :type Integer) (bFromSweep :type Boolean) (SweepResult :type "HitResult Structure (by ref)"))
  (`KismetSystemLibrary.PrintString` (`KismetSystemLibrary.GetObjectName` OtherActor)))

(fn `MoveTowards`
  (params (B :type "Vector Structure"))
  (`SceneComponent.K2_SetWorldLocation` (`self.Cube`) (`KismetMathLibrary.VLerp` (`SceneComponent.K2_GetComponentLocation` (`self.Cube`)) B 0.006) true false))

(fn `UserConstructionScript`
  (`parent.UserConstructionScript`))