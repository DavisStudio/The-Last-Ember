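; BP_Weapon is a tool actor that damages destroyable props it overlaps while the player is able to axe-swing.
; On overlap it checks CanAxeSwing on player character 0 and its own CanDamage, then calls TakeDamage on the BP_DestroyableProp.
; A hit clears CanDamage, which is not re-enabled here, and calls the empty PropHitY function.
; GivePlayerRef stores a player reference, but the overlap logic looks the player up directly.
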(event `self.ReceiveActorBeginOverlap`
  (params (OtherActor :type "Actor Object Reference"))
  (bind _asbp_charachter (cast `/Game/Charachter/BP_Charachter` (`GameplayStatics.GetPlayerCharacter` 0)))
  (if (and (`/Game/Charachter/BP_Charachter.CanAxeSwing` _asbp_charachter) (`self.CanDamage`))
    (bind _asbp_destroyable_prop (cast `/Game/BluePrints/InWorldProps/BP_DestroyableProp` OtherActor))
    (`/Game/BluePrints/InWorldProps/BP_DestroyableProp.TakeDamage` _asbp_destroyable_prop (`self.Damage`))
    (set `self.CanDamage` false)
    (`self.Prop Hit Y`)
    (else
      (`KismetSystemLibrary.PrintString` "1Hello"))))

(fn `GivePlayerRef`
  (params (PlayerRef :type "/Game/Charachter/BP_Charachter Object Reference"))
  (set `self.Player` PlayerRef))

(fn `Prop Hit Y`)

(fn `UserConstructionScript`)