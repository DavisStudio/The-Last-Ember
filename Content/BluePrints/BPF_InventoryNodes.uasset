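; Blueprint function library of inventory helpers for item totals and NPC quest item checks.
; Item stacks are summed into maps keyed by ID or class, and required-item class maps convert to ID keys through class defaults.
; CanCompleteQuest uses the ID totals to check that every required item is present, ignoring quantities.
; RemoveItems returns only the remaining amounts for the requested classes; its inventory-rebuilding branches are disconnected.
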(fn `CanCompleteQuest`
  (params (Inventory :type "Array of /Game/BluePrints/Structs/ST_Item Structure") (NPC_Info :type "/Game/BluePrints/Structs/ST_NPC Structure"))
  (returns (canHandInQuest :type Boolean))
  (locals (AmountOfItemsNeeded :type Integer) (PlayersINV :type "Map of Integer to Integer") (Matches :type Integer))
  (bind _iteminvoutput (`self.GetTotalItemAmount` Inventory))
  (set `local.PlayersINV` _iteminvoutput)
  (set `local.AmountOfItemsNeeded` (`BlueprintMapLibrary.Map_Length` NPC_Info_RequiredItems_37_243DFA824926F68D41E8349226D400FC))
  (bind _keys (`BlueprintMapLibrary.Map_Keys` NPC_Info_RequiredItems_37_243DFA824926F68D41E8349226D400FC))
  (bind _values (`BlueprintMapLibrary.Map_Values` NPC_Info_RewardItems_39_62DE02414FCA8FA1A197B1A3FD0D8C35))
  (for (_array_element _array_index) _keys
    (bind _properties_id (break `/Game/BluePrints/Structs/ST_Item` (defaults `Object` _array_element)))
    (if (`.ReturnValue` (`BlueprintMapLibrary.Map_Find` (`local.PlayersINV`) _properties_id))
      (`/Engine/EditorBlueprintResources/StandardMacros.IncrementInt` (`local.Matches`))))
  (if (== (`local.AmountOfItemsNeeded`) (`local.Matches`))
    (return true)
    (else
      (return false))))

(fn `convertNPCRequiredToMap`
  (params (RequiredItems :type "Map of /Game/BluePrints/Items/BP_Item Class Reference to Integer"))
  (returns (InvMap :type "Map of Integer to Integer"))
  (locals (RequiredItem :type "Map of /Game/BluePrints/Items/BP_Item Class Reference to Integer") (newInv :type "Map of Integer to Object Object Reference"))
  (bind _keys (`BlueprintMapLibrary.Map_Keys` RequiredItems))
  (for _array_element _keys
    (bind _properties_id (break `/Game/BluePrints/Structs/ST_Item` (defaults `Object` _array_element)))
    (`BlueprintMapLibrary.Map_Add` (`local.newInv`) _properties_id (`BlueprintMapLibrary.Map_Find` (`local.RequiredItems`) _array_element)))
  (return (`local.newInv`)))

(fn `GetTotalItemAmount`
  (params (Inventory :type "Array of /Game/BluePrints/Structs/ST_Item Structure"))
  (returns (ItemInvOutput :type "Map of Integer to Integer"))
  (locals (`Item_ID-AMOUNT` :type "Map of Integer to Integer"))
  (bind _item_id_amount (`local.Item_ID-AMOUNT`))
  (bind _item_id_amount_2 (`local.Item_ID-AMOUNT`))
  (for _array_element Inventory
    (bind (_id _rarity _name _type _icon _maxstacksize _amount) (break `/Game/BluePrints/Structs/ST_Item` _array_element))
    (if (`BlueprintMapLibrary.Map_Contains` _item_id_amount _id)
      (`BlueprintMapLibrary.Map_Add` _item_id_amount_2 _id (+ (`BlueprintMapLibrary.Map_Find` _item_id_amount _id) _amount))
      (else
        (`BlueprintMapLibrary.Map_Add` _item_id_amount_2 _id _amount))))
  (return (`local.Item_ID-AMOUNT`)))

(fn `GetTotalItemAmount_CLASSREF`
  (params (Inventory :type "Array of /Game/BluePrints/Structs/ST_Item Structure"))
  (returns (ItemInvOutput :type "Map of /Game/BluePrints/Items/BP_Item Class Reference to Integer"))
  (locals (`Item_ID-AMOUNT` :type "Map of /Game/BluePrints/Items/BP_Item Class Reference to Integer"))
  (bind _item_id_amount (`local.Item_ID-AMOUNT`))
  (bind _item_id_amount_2 (`local.Item_ID-AMOUNT`))
  (for _array_element Inventory
    (bind (_id _rarity _name _type _icon _maxstacksize _amount _selfreff) (break `/Game/BluePrints/Structs/ST_Item` _array_element))
    (if (`BlueprintMapLibrary.Map_Contains` _item_id_amount _selfreff)
      (`BlueprintMapLibrary.Map_Add` _item_id_amount_2 _selfreff (+ (`BlueprintMapLibrary.Map_Find` _item_id_amount _selfreff) _amount))
      (else
        (`BlueprintMapLibrary.Map_Add` _item_id_amount_2 _selfreff _amount))))
  (return (`local.Item_ID-AMOUNT`)))

(fn `removeItems`
  (params (ItemsToRemove :type "Map of /Game/BluePrints/Items/BP_Item Class Reference to Integer") (Inventory :type "Array of /Game/BluePrints/Structs/ST_Item Structure"))
  (returns (NewINVR :type "Map of /Game/BluePrints/Items/BP_Item Class Reference to Integer") (newInvOutput1 :type "Array of /Game/BluePrints/Structs/ST_Item Structure"))
  (locals (newInv :type "Map of /Game/BluePrints/Items/BP_Item Class Reference to Integer") (inv :type "Array of /Game/BluePrints/Structs/ST_Item Structure") (newInvOutput :type "Array of /Game/BluePrints/Structs/ST_Item Structure") (OverFlow :type Integer))
  (set `local.inv` Inventory)
  (bind _iteminvoutput (`self.GetTotalItemAmount` Inventory))
  (bind _keys (`BlueprintMapLibrary.Map_Keys` ItemsToRemove))
  (for _array_element _keys
    (`BlueprintMapLibrary.Map_Add` (`local.newInv`) _array_element (- (`BlueprintMapLibrary.Map_Find` _iteminvoutput (`.ID_2_86D9E0774AE908F18D54DCB6E4B8268F` (break `/Game/BluePrints/Structs/ST_Item` (defaults `Object` _array_element)))) (`BlueprintMapLibrary.Map_Find` ItemsToRemove _array_element))))
  (return (`local.newInv`)))