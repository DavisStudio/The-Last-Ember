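; Child NPC Blueprint, named for a swamp gate, that runs a two-stage quest interaction keyed on CurrentQuest.
; It stores the player and enables interaction when the matching QuestsDone flag is set, hiding the exclamation marker in stage two.
; Accepting sets a flag and disables interaction.
; Handing in lowers player max health and sets a flag; stage two also rebuilds a house and moves the text box zone.
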(event `self.ReceiveBeginPlay`
  (`parent.ReceiveBeginPlay`)
  (set `self.CanInteract` true))

(event `self.ReceiveTick`
  (params (DeltaSeconds :type "Float (single-precision)"))
  (`parent.ReceiveTick` DeltaSeconds))

(event `/Game/BluePrints/BPI_QuestUpdates.HandInQuest`
  (params (NPC :type "/Game/BluePrints/Structs/ST_NPC Structure"))
  (bind _playerref (`self.PlayerRef`))
  (bind _playermaxhealh (`/Game/Charachter/BP_Charachter.PlayerMaxHealh` _playerref))
  (switch `int` (`self.CurrentQuest`)
    (:`0`
      (set `/Game/Charachter/BP_Charachter.PlayerMaxHealh` (- _playermaxhealh 0.1) _playerref)
      (`KismetArrayLibrary.Array_Set` (`/Game/Charachter/BP_Charachter.QuestsDone` (`self.PlayerRef`)) 0 true))
    (:`1`
      (`/Game/BluePrints/InWorldProps/QuestRewardBuildigns/BP_RockNPCHouse.RebuildStructure` (`self.HosueRef`))
      (set `/Game/Charachter/BP_Charachter.PlayerMaxHealh` (- _playermaxhealh 0.25) _playerref)
      (`KismetArrayLibrary.Array_Set` (`/Game/Charachter/BP_Charachter.QuestsDone` (`self.PlayerRef`)) 3 true)
      (`SceneComponent.K2_SetWorldLocation` (`self.BP_TextBoxZone`) (`SceneComponent.K2_GetComponentLocation` (`self.Cube`)) false true))))

(event `Key|F`
  (params (Key :type "Key Structure")))

(event `/Game/BluePrints/BPI_QuestUpdates.NPC_AcceptQuestINt`
  (params (NewParam :type "/Game/Charachter/BP_Charachter Object Reference"))
  (`KismetArrayLibrary.Array_Set` (`/Game/Charachter/BP_Charachter.QuestsDone` NewParam) 0 true)
  (set `self.CanInteract` false))

(event `/Game/BluePrints/BPI_QuestUpdates.CheckIfcanInteract`
  (params (player :type "/Game/Charachter/BP_Charachter Object Reference"))
  (bind _output_get (set `self.PlayerRef` player))
  (for (_array_element _array_index) (`/Game/Charachter/BP_Charachter.QuestsDone` _output_get)
    (switch `int` (`self.CurrentQuest`)
      (:`0`
        (if (and _array_element (== _array_index 0))
          (set `self.CanInteract` true)))
      (:`1`
        (if (and _array_element (== _array_index 1))
          (set `self.CanInteract` true)
          (`SceneComponent.SetVisibility` (`self.BP_Exlamation`) false false))))))

(fn `UserConstructionScript`
  (`parent.UserConstructionScript`))