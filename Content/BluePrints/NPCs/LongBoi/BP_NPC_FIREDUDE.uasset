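; Quest NPC "Fire Dude", who blinks periodically through a timeline-driven material parameter and becomes interactable once the player's first quest flag is done.
; Accepting his first quest calls the player's quest hand-in with Marie as the NPC reference.
; Handing it in flags progress, repairs the workshop, spawns an axe with sawing and hammering sounds, and lowers player max health.
; His second hand-in only sets the next completion flag.
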(event `self.ReceiveBeginPlay`
  (`parent.ReceiveBeginPlay`))

(event `self.ReceiveTick`
  (params (DeltaSeconds :type "Float (single-precision)"))
  (`parent.ReceiveTick` DeltaSeconds)
  (`KismetSystemLibrary.Delay` (`KismetMathLibrary.RandomFloatInRange` 4.0 8.0))
  (bind (_direction _newtrack_0) (`Timeline|Blink` :!via `PlayFromStart`)
    (:`Update`
      (`MeshComponent.SetScalarParameterValueOnMaterials` (`self.Cube`) "Blink" _newtrack_0))))

(event `/Game/BluePrints/BPI_QuestUpdates.ReadyToHandIn`
  (params (QuestIndex :type Integer) (QuestID :type Integer))
  (if (== (`.QuestID_4_5DFF6F654F8A3761B576419BD4ABD02D` (break `/Game/BluePrints/Structs/ST_NPC` (`|GetArrayItem` (`self.QuestInfo`) (`self.CurrentQuest`)))) QuestID)
    _))

(event `/Game/BluePrints/BPI_QuestUpdates.HandInQuest`
  (params (NPC :type "/Game/BluePrints/Structs/ST_NPC Structure"))
  (bind _playerref (`self.PlayerRef`))
  (bind _returnvalue (`SceneComponent.K2_GetComponentLocation` (`self.Cube1`)))
  (switch `int` (`self.CurrentQuest`)
    (:`0`
      (bind _asbp_charachter (cast `/Game/Charachter/BP_Charachter` (`GameplayStatics.GetPlayerCharacter` 0)))
      (`KismetArrayLibrary.Array_Set` (`/Game/Charachter/BP_Charachter.QuestsDone` _asbp_charachter) 1 true)
      (`/Game/Assets/WorkShop/BP_WorkShop.RepairWorkShop` (`self.WorkShop`))
      (`|SpawnActorFromClass` "/Game/BluePrints/Items/BP_Item_AXE.BP_Item_AXE_C" (`SceneComponent.K2_GetComponentToWorld` (`self.Cube1`)) "AlwaysSpawn" "OverrideRootScale" null null)
      (set `/Game/Charachter/BP_Charachter.PlayerMaxHealh` (- (`/Game/Charachter/BP_Charachter.PlayerMaxHealh` _playerref) 0.15) _playerref)
      (`GameplayStatics.PlaySoundAtLocation` "/Game/Sounds/newSounds/SawCut.SawCut" _returnvalue (struct) 1.0 1.0 0.0 null null null)
      (`GameplayStatics.PlaySoundAtLocation` "/Game/Sounds/newSounds/HamerHit.HamerHit" _returnvalue (struct) 1.0 1.0 0.0 null null null))
    (:`1`
      (bind _asbp_charachter_2 (cast `/Game/Charachter/BP_Charachter` (`GameplayStatics.GetPlayerCharacter` 0)))
      (`KismetArrayLibrary.Array_Set` (`/Game/Charachter/BP_Charachter.QuestsDone` _asbp_charachter_2) 2 true))))

(event `/Game/BluePrints/BPI_QuestUpdates.QuestAccepted_NPC`
  (switch `int` (`self.CurrentQuest`)
    (:`0`
      (bind _asbp_charachter (cast `/Game/Charachter/BP_Charachter` (`GameplayStatics.GetPlayerCharacter` 0)))
      (`/Game/BluePrints/BPI_QuestUpdates.HandInQuest` _asbp_charachter (make `/Game/BluePrints/Structs/ST_NPC` :`QuestID` 5 :`NPC_Ref` (`self.Marie`))))))

(event `/Game/BluePrints/BPI_QuestUpdates.CheckIfcanInteract`
  (params (player :type "/Game/Charachter/BP_Charachter Object Reference"))
  (bind _output_get (set `self.PlayerRef` player))
  (for (_array_element _array_index) (`/Game/Charachter/BP_Charachter.QuestsDone` _output_get)
    (if (and (== _array_index 0) _array_element)
      (set `self.CanInteract` true))))

(fn `UserConstructionScript`
  (`parent.UserConstructionScript`))