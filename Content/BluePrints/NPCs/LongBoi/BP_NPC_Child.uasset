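; Child NPC Blueprint for Long Robe Larry, a quest character whose interaction depends on the player's completed quests.
; On BeginPlay it gathers leaf, twig and rock components, and a timeline moves Larry along Z while clearing CanInteract.
; CheckIfcanInteract re-enables interaction for quest 0 when QuestsDone index 1 is true.
; Boundary overlaps toggle a gate for rotating the debris, but its Enter is unreachable; Tick debug-prints CurrentQuest.
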(event `self.ReceiveBeginPlay`
  (`parent.ReceiveBeginPlay`)
  (set `self.Leafs` (`|MakeArray` (`self.Leaves_FBX_Leaf6`) (`self.Leaves_FBX_Twig2`) (`self.Leaves_FBX_Twig1`) (`self.Leaves_FBX_SmallRock`) (`self.Leaves_FBX_MedRock`) (`self.Leaves_FBX_BigRock`) (`self.Leaves_FBX_Leaf5`) (`self.Leaves_FBX_Leaf4`) (`self.Leaves_FBX_Leaf3`) (`self.Leaves_FBX_Leaf2`) (`self.Leaves_FBX_Leaf1`)))
  (bind (_direction _newtrack_3) (`Timeline|Timeline_0`)
    (:`Update`
      (`SceneComponent.K2_SetRelativeLocation` (`self.LONGROBELARRYANIMATED`) (`KismetMathLibrary.MakeVector` 0.0 0.0 (`KismetMathLibrary.Lerp` (`self.StartPoint`) (`self.EndPoint`) _newtrack_3)) false false)
      (set `self.CanInteract` false))))

(event `self.BoundaryPlayerTracker.OnComponentBeginOverlap`
  (params (OverlappedComponent :type "PrimitiveComponent Object Reference") (OtherActor :type "Actor Object Reference") (OtherComp :type "PrimitiveComponent Object Reference") (OtherBodyIndex :type Integer) (bFromSweep :type Boolean) (SweepResult :type "HitResult Structure (by ref)"))
  (`/Engine/EditorBlueprintResources/StandardMacros.Gate` true :!via `Open` :!label _label
    (:`Exit`
      (for _array_element (`self.Leafs`)
        (`SceneComponent.K2_AddWorldRotation` _array_element (struct :`Yaw` 20.0) false false)))))

(event `self.BoundaryPlayerTracker.OnComponentEndOverlap`
  (params (OverlappedComponent :type "PrimitiveComponent Object Reference") (OtherActor :type "Actor Object Reference") (OtherComp :type "PrimitiveComponent Object Reference") (OtherBodyIndex :type Integer))
  (goto _label :!via `Close`))

(event `/Game/BluePrints/BPI_QuestUpdates.HandInQuest`
  (params (NPC :type "/Game/BluePrints/Structs/ST_NPC Structure")))

(event `self.ReceiveTick`
  (params (DeltaSeconds :type "Float (single-precision)"))
  (`KismetSystemLibrary.PrintString` (`KismetStringLibrary.Conv_IntToString` (`self.CurrentQuest`))))

(event `/Game/BluePrints/BPI_QuestUpdates.CheckIfcanInteract`
  (params (player :type "/Game/Charachter/BP_Charachter Object Reference"))
  (for (_array_element _array_index) (`/Game/Charachter/BP_Charachter.QuestsDone` player)
    (switch `int` (`self.CurrentQuest`)
      (:`0`
        (if (and _array_element (== _array_index 1))
          (set `self.CanInteract` true))))))

(fn `UserConstructionScript`
  (`parent.UserConstructionScript`))