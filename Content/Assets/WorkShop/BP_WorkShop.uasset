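; BP_WorkShop is a repairable workshop that starts with its anvil, work table and furnace hidden and non-collidable.
; RepairWorkShop activates a building dust particle effect and plays a timeline that fades four point lights up to a configurable maximum intensity.
; Once the timeline track passes 0.7 the props become visible with collision, masked by the dust, which deactivates when the timeline finishes.
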(event `self.ReceiveBeginPlay`
  (bind _output_get (set `self.Props` (`|MakeArray` (`self.Anvil_FBX`) (`self.Work_Table_FBX`) (`self.Furnace_FBX`))))
  (for _array_element _output_get
    (`PrimitiveComponent.SetCollisionEnabled` _array_element "NoCollision")
    (`SceneComponent.SetVisibility` _array_element false true)
    (`ActorComponent.Deactivate` (`self.PS_BuildingDustWorkshop`))))

(event `RepairWorkShop`
  (`ActorComponent.Activate` (`self.PS_BuildingDustWorkshop`) false)
  (bind (_direction _newtrack_0) (`Timeline|Timeline_0` :!via `PlayFromStart`)
    (:`Update`
      (if (< 0.7 _newtrack_0)
        (for _array_element (`self.Props`)
          (`PrimitiveComponent.SetCollisionEnabled` _array_element "QueryAndPhysics")
          (`SceneComponent.SetVisibility` _array_element true true)))
      (for _array_element_2 (`|MakeArray` (`self.PointLight2`) (`self.PointLight3`) (`self.PointLight`) (`self.PointLight1`))
        (`LightComponent.SetIntensity` _array_element_2 (`KismetMathLibrary.Lerp` 0.0 (`self.MaxIntesityFading lights`) _newtrack_0))))
    (:`Finished`
      (`ActorComponent.Deactivate` (`self.PS_BuildingDustWorkshop`)))))

(fn `UserConstructionScript`)